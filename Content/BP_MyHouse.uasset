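; BP_MyHouse is a practice house Blueprint whose live logic only exercises two variables.
; BeginPlay prints and reassigns MyFirstVar and MySecondVar, showing their values on screen.
; A disconnected EventGraph chain would assemble a house by adding scaled cube static mesh components for base and walls, plus two ramp meshes.
; That chain never runs and the construction script is empty, so this logic builds no house.
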(event `self.ReceiveBeginPlay`
  (`KismetSystemLibrary.PrintString` (`KismetStringLibrary.Conv_IntToString` (`self.myFirstVar`)))
  (bind _output_get (set `self.myFirstVar` 2))
  (`KismetSystemLibrary.PrintString` (`KismetStringLibrary.Concat_StrStr` (`KismetStringLibrary.Conv_IntToString` _output_get)))
  (`KismetSystemLibrary.PrintString` (`KismetStringLibrary.Conv_DoubleToString` (`self.mySecondVar`)))
  (bind _output_get_2 (set `self.mySecondVar` 4.0))
  (`KismetSystemLibrary.PrintString` (`KismetStringLibrary.Conv_DoubleToString` _output_get_2)))

(fn `UserConstructionScript`)